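; BP_Door is a door actor that serves as the win trigger for the third-person character.
; On BeginPlay it caches the player's pawn, cast to BP_ThirdPersonCharacter.
; Any overlap with its Box component sets IsWin on that character if CountDown converts to true, without checking which actor entered.
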(event `self.ReceiveBeginPlay`
  (`self.create player`))

(event `self.Box.OnComponentBeginOverlap`
  (params (OverlappedComponent :type "PrimitiveComponent Object Reference") (OtherActor :type "Actor Object Reference") (OtherComp :type "PrimitiveComponent Object Reference") (OtherBodyIndex :type Integer) (bFromSweep :type Boolean) (SweepResult :type "HitResult Structure (by ref)"))
  (bind _as_bp_third_person_character (`self.As BP Third Person Character`))
  (if (`KismetMathLibrary.Conv_IntToBool` (`/Game/ThirdPerson/Blueprints/BP_ThirdPersonCharacter.Count_Down` _as_bp_third_person_character))
    (set `/Game/ThirdPerson/Blueprints/BP_ThirdPersonCharacter.Is_Win` true _as_bp_third_person_character)))

(event `create player`
  (bind _asbp_third_person_character (cast `/Game/ThirdPerson/Blueprints/BP_ThirdPersonCharacter` (`Controller.K2_GetPawn` (`GameplayStatics.GetPlayerController` 0))))
  (set `self.As BP Third Person Character` _asbp_third_person_character))

(fn `UserConstructionScript`)