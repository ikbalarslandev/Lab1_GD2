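; BP_MazeCell is one maze cell that builds its own ground, walls, ceiling and light at BeginPlay.
; It scales the ground from GridSize, then spawns scaled BP_Cube actors at marker points for each enabled wall and the ceiling.
; A ceiling also spawns a configurable point light.
; Each Tick it polls the player character, turning that light green on a win or red when CountDown runs out, and printing the result.
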(event `create player`
  (bind _asbp_third_person_character (cast `/Game/ThirdPerson/Blueprints/BP_ThirdPersonCharacter` (`Controller.K2_GetPawn` (`GameplayStatics.GetPlayerController` 0))))
  (set `self.As BP Third Person Character` _asbp_third_person_character))

(event `self.ReceiveBeginPlay`
  (bind _grid_scale_size (`self.Grid_Scale_Size`))
  (bind _grid_scale_size_2 (`self.Grid_Scale_Size`))
  (bind _grid_scale_size_3 (`self.Grid_Scale_Size`))
  (bind _grid_scale_size_4 (`self.Grid_Scale_Size`))
  (bind _grid_scale_size_5 (`self.Grid_Scale_Size`))
  (bind _grid_scale_size_6 (`self.Grid_Scale_Size`))
  (bind (_returnvalue_x _returnvalue_y _returnvalue_z) (`KismetMathLibrary.BreakVector` (`SceneComponent.K2_GetComponentLocation` (`self.East_Point`))))
  (bind (_returnvalue_x_2 _returnvalue_y_2 _returnvalue_z_2) (`KismetMathLibrary.BreakVector` (`SceneComponent.K2_GetComponentLocation` (`self.West_Point`))))
  (bind (_returnvalue_x_3 _returnvalue_y_3 _returnvalue_z_3) (`KismetMathLibrary.BreakVector` (`SceneComponent.K2_GetComponentLocation` (`self.South_Point`))))
  (bind (_returnvalue_x_4 _returnvalue_y_4 _returnvalue_z_4) (`KismetMathLibrary.BreakVector` (`SceneComponent.K2_GetComponentLocation` (`self.Ceiling_Point`))))
  (bind (_returnvalue_x_5 _returnvalue_y_5 _returnvalue_z_5) (`KismetMathLibrary.BreakVector` (`SceneComponent.K2_GetComponentLocation` (`self.North_Point`))))
  (`self.create player`)
  ; Set Grid Scale Size
  (set `self.Grid_Scale_Size` (/ (`self.GridSize`) 100.0))
  ; Set Ground
  (`SceneComponent.SetWorldScale3D` (`self.Cube`) (`KismetMathLibrary.MakeVector` _grid_scale_size_6 _grid_scale_size_6 (/ _grid_scale_size_6 10.0)))
  ; Set East Wall
  (if (`self.EastWall`)
    (`|SpawnActorFromClass` "/Game/BP_Cube.BP_Cube_C" (`KismetMathLibrary.MakeTransform` (`KismetMathLibrary.MakeVector` _returnvalue_x _returnvalue_y (+ _returnvalue_z (/ (`self.GridSize`) 2.0))) (struct) (`KismetMathLibrary.MakeVector` (* _grid_scale_size 0.1) _grid_scale_size _grid_scale_size)) "Undefined" "MultiplyWithRoot" null null))
  ; Set West Wall
  (if (`self.WestWall`)
    (`|SpawnActorFromClass` "/Game/BP_Cube.BP_Cube_C" (`KismetMathLibrary.MakeTransform` (`KismetMathLibrary.MakeVector` _returnvalue_x_2 _returnvalue_y_2 (+ _returnvalue_z_2 (/ (`self.GridSize`) 2.0))) (struct) (`KismetMathLibrary.MakeVector` (* _grid_scale_size_2 0.1) _grid_scale_size_2 _grid_scale_size_2)) "Undefined" "MultiplyWithRoot" null null))
  ; Set South Wall
  (if (`self.SouthWall`)
    (`|SpawnActorFromClass` "/Game/BP_Cube.BP_Cube_C" (`KismetMathLibrary.MakeTransform` (`KismetMathLibrary.MakeVector` _returnvalue_x_3 _returnvalue_y_3 (+ _returnvalue_z_3 (/ (`self.GridSize`) 2.0))) (struct) (`KismetMathLibrary.MakeVector` _grid_scale_size_3 (* _grid_scale_size_3 0.1) _grid_scale_size_3)) "Undefined" "MultiplyWithRoot" null null))
  ; Set North Wall
  (if (`self.NorthWall`)
    (`|SpawnActorFromClass` "/Game/BP_Cube.BP_Cube_C" (`KismetMathLibrary.MakeTransform` (`KismetMathLibrary.MakeVector` _returnvalue_x_5 _returnvalue_y_5 (+ _returnvalue_z_5 (/ (`self.GridSize`) 2.0))) (struct) (`KismetMathLibrary.MakeVector` _grid_scale_size_4 (* _grid_scale_size_4 0.1) _grid_scale_size_4)) "Undefined" "MultiplyWithRoot" null null))
  ; Set Ceiling
  (if (`self.Ceiling`)
    (bind _returnvalue (`|SpawnActorFromClass` "/Game/BP_Cube.BP_Cube_C" (`KismetMathLibrary.MakeTransform` (`KismetMathLibrary.MakeVector` _returnvalue_x_4 _returnvalue_y_4 (+ _returnvalue_z_4 (* (`self.GridSize`) 0.9))) (struct) (`KismetMathLibrary.MakeVector` _grid_scale_size_5 _grid_scale_size_5 (* _grid_scale_size_5 0.1))) "Undefined" "MultiplyWithRoot" null null))
    (bind _returnvalue_2 (`|SpawnActorFromClass` "/Script/Engine.PointLight" (`KismetMathLibrary.MakeTransform` (`self.K2_GetActorLocation` _returnvalue)) "Undefined" "MultiplyWithRoot" null null))
    (set `self.Point_Light` _returnvalue_2)
    (bind _pointlightcomponent (`PointLight.PointLightComponent` _returnvalue_2))
    (`LightComponent.SetIntensity` _pointlightcomponent (`self.Light_Intensity`))
    (`LightComponent.SetLightColor` _pointlightcomponent (`self.Light_Color`) true)))

(event `self.ReceiveTick`
  (params (DeltaSeconds :type "Float (single-precision)"))
  (bind _as_bp_third_person_character (`self.As BP Third Person Character`))
  (if (`/Game/ThirdPerson/Blueprints/BP_ThirdPersonCharacter.Is_Win` _as_bp_third_person_character)
    (`LightComponent.SetLightColor` (`Light.LightComponent` (`self.Point_Light`)) (struct :`R` 0.021945 :`G` 1.0 :`A` 1.0) true)
    (`KismetSystemLibrary.PrintString` "Well Done!!")
    (elif (`KismetMathLibrary.Conv_IntToBool` (`/Game/ThirdPerson/Blueprints/BP_ThirdPersonCharacter.Count_Down` _as_bp_third_person_character))
      _
      (elif (not (`/Game/ThirdPerson/Blueprints/BP_ThirdPersonCharacter.Is_Win` _as_bp_third_person_character))
        (`LightComponent.SetLightColor` (`Light.LightComponent` (`self.Point_Light`)) (struct :`R` 1.0 :`B` 0.023948 :`A` 1.0) true)
        (`KismetSystemLibrary.PrintString` "You Have Failed")))))

(fn `UserConstructionScript`)